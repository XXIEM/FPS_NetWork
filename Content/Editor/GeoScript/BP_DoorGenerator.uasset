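; Editor Geometry Script generator that builds a door mesh as a box with a box-shaped cut subtracted from it.
; On rebuild, it appends a subdivided box from Size, then subtracts a pooled tool box placed at Pivot and sized by CalSizeAndLocation.
; The result gets a polygroup bevel and a complex-as-simple collision setting, then all pooled meshes are returned.
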(event `self.OnRebuildGeneratedMesh`
  (params (TargetMesh :type "DynamicMesh Object Reference"))
  (bind (_size_x _size_y _size_z) (`KismetMathLibrary.BreakVector` (`self.Size`)))
  (bind _returnvalue (- (`self.ControlPoint`) (`self.Pivot`)))
  (bind (_returnvalue_x _returnvalue_y _returnvalue_z) (`KismetMathLibrary.BreakVector` (`KismetMathLibrary.Vector_GetAbs` (* _returnvalue (2.0 2.0 1.0)))))
  (set `self.Target Mesh` TargetMesh)
  (bind _returnvalue_2 (`self.GetComputeMeshPool`))
  (set `self.Pool` _returnvalue_2)
  (`|ExecutionSequence`
    (:`then_0`
      (`GeometryScriptLibrary_MeshPrimitiveFunctions.AppendBox` (`self.Target Mesh`) (struct) (struct) _size_x _size_y _size_z 5 5 5 "Base" null))
    (:`then_1`
      (bind _returnvalue_3 (`DynamicMeshPool.RequestMesh` (`self.Pool`)))
      (bind _returnvalue_4 (`GeometryScriptLibrary_MeshPrimitiveFunctions.AppendBox` _returnvalue_3 (struct) (`KismetMathLibrary.MakeTransform` (`self.Pivot`) (struct) (`KismetMathLibrary.Vector_GetSignVector` _returnvalue)) _returnvalue_x _returnvalue_y _returnvalue_z 0 0 0 "Base" null))
      (bind _returnvalue_5 (`GeometryScriptLibrary_MeshBooleanFunctions.ApplyMeshBoolean` (`self.Target Mesh`) (struct) _returnvalue_4 (struct) "Subtract" (struct) null))
      (`GeometryScriptLibrary_MeshModelingFunctions.ApplyMeshPolygroupBevel` _returnvalue_5 (make `GeometryScriptMeshBevelOptions` (`self.BevelDistance`)) null))
    (:`then_2`
      (`DynamicMeshComponent.SetComplexAsSimpleCollisionEnabled` (`self.DynamicMeshComponent`) (`self.UseComplexCollision`) true))
    (:`then_3`
      (`DynamicMeshPool.ReturnAllMeshes` (`self.Pool`)))))

(fn `UserConstructionScript`)