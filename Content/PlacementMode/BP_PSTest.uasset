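; BP_PSTest is a small test Blueprint for placement mode that works through the player controller.
; On BeginPlay it shows the mouse cursor when a player controller is valid.
; An unconnected debug chain would print the count of the first placement actor item from PlacementPSComponent for the local controller.
; Tick does nothing, and the construction script only calls its parent.
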(event `self.ReceiveBeginPlay`
  (bind _returnvalue (`self.GetPlayerController`))
  (`/Engine/EditorBlueprintResources/StandardMacros.IsValid` _returnvalue
    (:`Is Valid`
      (set `PlayerController.bShowMouseCursor` true _returnvalue))))

(event `self.ReceiveTick`
  (params (DeltaSeconds :type "Float (single-precision)")))

(fn `UserConstructionScript`
  (`parent.UserConstructionScript`))