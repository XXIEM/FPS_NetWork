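; Test placement actor for placement mode that shows or hides its static mesh as the placement state changes.
; The state change event always shows the mesh when placed and, when unplaced, shows it only if the spawner is the local player controller.
; The construction script lifts the mesh by its local minimum Z bound so its base sits at the actor origin.
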(event `self.ReceiveBeginPlay`
  (`parent.ReceiveBeginPlay`))

(event `self.OnStateChange`
  (params (State :type "EPlacementActorStateType Enum" :default "Place") (InSpawner :type "Actor Object Reference"))
  (bind _staticmesh (`self.StaticMesh`))
  (switch `EPlacementActorStateType` State
    (:`Place`
      (`SceneComponent.SetVisibility` _staticmesh true false))
    (:`UnPlace`
      (`SceneComponent.SetVisibility` _staticmesh (== InSpawner (`GameplayStatics.GetPlayerController` 0)) false))))

(fn `UserConstructionScript`
  (bind _staticmesh (`self.StaticMesh`))
  (`parent.UserConstructionScript`)
  (`SceneComponent.K2_AddLocalOffset` _staticmesh (`KismetMathLibrary.MakeVector` 0.0 0.0 (* (`.Z` (`KismetMathLibrary.BreakVector3f` (`StaticMeshComponent.GetLocalBounds` _staticmesh))) -1.0)) false false))