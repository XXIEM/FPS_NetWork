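; Placement-mode pipeline generator that procedurally builds an open-ended pipe mesh along a spline with Geometry Script.
; On mesh rebuild, it caches the target mesh and sweeps a circle along sampled spline frames, using radius and resolution from Info.
; It flips the normals, then boolean-subtracts the cached mesh of each BoolenTarget entry from the pipe.
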(event `self.OnRebuildGeneratedMesh`
  (params (TargetMesh :type "DynamicMesh Object Reference"))
  (bind _info_splinepointnum (break `/Game/PlacementMode/S_PipelineInfo` (`self.Info`)))
  (bind (_info_splinepointnum_2 _info_pipelineradius _info_pipelinepointnum) (break `/Game/PlacementMode/S_PipelineInfo` (`self.Info`)))
  (set `self.Target Mesh` TargetMesh)
  (bind _frames (`GeometryScriptLibrary_PolyPathFunctions.SampleSplineToTransforms` (`self.Spline`) (make `GeometryScriptSplineSamplingOptions` _info_splinepointnum)))
  (bind _returnvalue (`GeometryScriptLibrary_PolyPathFunctions.CreateCirclePath2D` (0.0 0.0) _info_pipelineradius _info_pipelinepointnum))
  (bind _returnvalue_2 (`GeometryScriptLibrary_MeshPrimitiveFunctions.AppendSweepPolygon` (`self.Target Mesh`) (struct) (struct) (`GeometryScriptLibrary_PolyPathFunctions.Conv_GeometryScriptPolyPathToArrayOfVector2D` _returnvalue) _frames false false 1.0 1.0 0.0 null))
  (`GeometryScriptLibrary_MeshNormalsFunctions.FlipNormals` _returnvalue_2 null)
  (for _array_element (`self.BoolenTarget`)
    (`GeometryScriptLibrary_MeshBooleanFunctions.ApplyMeshBoolean` (`self.Target Mesh`) (struct) (`/Game/PlacementMode/BP_PipelineGenerator.Target Mesh` _array_element) (struct) "Subtract" (struct) null)))

(fn `UserConstructionScript`)