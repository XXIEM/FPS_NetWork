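; Base weapon Blueprint that drives shooting recoil on the main character and refreshes the ammo UI.
; AddRecoil plays a timeline feeding yaw and pitch input from a RecoilCurve sampled by shot count, tracking accumulated offsets.
; RecoilDown stops that climb and plays a Drop timeline returning the view by the tracked amounts.
; Tick eases a pitch-scaled gun kick offset through double interpolation and prints the bullet count; camera shake is unwired.
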(event `self.AddRecoil`
  (bind _maincharacter (`self.MainCharacter`))
  (bind _upmultiplier (`self.UpMultiplier`))
  (bind _returnvalue_x (`KismetMathLibrary.BreakVector` (`CurveVector.GetVectorValue` (`self.RecoilCurve`) (`KismetMathLibrary.Conv_IntToDouble` (`self.CurrentShootTimes`)))))
  (bind (_returnvalue_x_2 _returnvalue_y) (`KismetMathLibrary.BreakVector` (`CurveVector.GetVectorValue` (`self.RecoilCurve`) (`KismetMathLibrary.Conv_IntToDouble` (`self.CurrentShootTimes`)))))
  (bind _returnvalue (* (* _returnvalue_y _upmultiplier) -1.0))
  (bind _returnvalue_2 (* (/ (* (* _returnvalue_x _upmultiplier) -1.0) 1.0) (`GameplayStatics.GetWorldDeltaSeconds`)))
  (bind _returnvalue_3 (* (/ _returnvalue 1.0) (`GameplayStatics.GetWorldDeltaSeconds`)))
  (`|ExecutionSequence`
    (:`then_0`
      ;[1 1 1] 后坐力上升
      (`Timeline|Timeline` :!via `PlayFromStart` :!label _label
        (:`Update`
          (`|ExecutionSequence`
            (:`then_0`
              (set `self.MaxRecoilX` (+ _returnvalue_2 (`self.MaxRecoilX`)))
              (`Pawn.AddControllerYawInput` _maincharacter _returnvalue_2))
            (:`then_1`
              (if (> (`self.MaxRecoilY`) _returnvalue)
                (set `self.MaxRecoilY` (+ _returnvalue_3 (`self.MaxRecoilY`)))
                (`Pawn.AddControllerPitchInput` _maincharacter _returnvalue_3)))))))
    (:`then_1`
      (`/Engine/EditorBlueprintResources/StandardMacros.IncrementInt` (`self.CurrentShootTimes`)))
    (:`then_2`
      (bind _output_get (set `self.Anim_TargetRecoil` (`KismetMathLibrary.MakeTransform` (`KismetMathLibrary.MakeVector` 0.0 (`KismetMathLibrary.MapRangeClamped` (`self.MaxRecoilY`) 0.0 -3.0 -4.0 -7.0)))))
      (set `self.Anim_CurrentRecoilOffset` _output_get))
    (:`then_3`
      ;[1 1 1] 弹药量UI更新
      (message `/Game/Game/Weapon/BPI_BulletRelord.RelordUpdate` (`MainCharacter.UI_Relord` (`self.MainCharacter`)) (`self.CurrentBulletNum`) (`self.TotalBulletNum`) :!label _label_2))))

(event `self.StopUp`
  ;[1 1 1] 后坐力上升
  (goto _label :!via `Stop`))

(event `StopUpBP`
  ;[1 1 1] 后坐力上升
  (goto _label :!via `Stop`))

(event `self.CallUIRelordUpdate`
  ;[1 1 1] 弹药量UI更新
  (goto _label_2))

(event `self.RecoilDown`
  (bind _dropavoidoffsetx (`self.DropAvoidOffsetX`))
  (bind _maxrecoilx (`self.MaxRecoilX`))
  (bind _maincharacter (`self.MainCharacter`))
  (bind _returnvalue (* (/ (`self.MaxRecoilX`) 0.27) (`GameplayStatics.GetWorldDeltaSeconds`)))
  (bind _returnvalue_2 (* (/ (`self.MaxRecoilY`) 0.27) (`GameplayStatics.GetWorldDeltaSeconds`)))
  (`|ExecutionSequence`
    (:`then_0`
      (`Pawn.AddControllerPitchInput` (`self.MainCharacter`) 0.0)
      (set `self.UpOneTime` 0.0)
      (set `self.LROneTime` 0.0))
    (:`then_1`
      ;[1 1 1] 后坐力回落
      (`Timeline|Drop` :!via `PlayFromStart` :!label _label_3
        (:`Update`
          (`|ExecutionSequence`
            (:`then_0`
              (if (< (`self.MaxRecoilX`) 0.0)
                (if (> _dropavoidoffsetx _maxrecoilx)
                  (set `self.DropAvoidOffsetX` (+ _returnvalue (`self.DropAvoidOffsetX`)) :!label _label_4)
                  (`Pawn.AddControllerYawInput` _maincharacter (* _returnvalue -1.0)))
                (elif (< _dropavoidoffsetx _maxrecoilx)
                  (goto _label_4))))
            (:`then_1`
              (if (> (`self.DropAvoidOffsetY`) (`self.MaxRecoilY`))
                (set `self.DropAvoidOffsetY` (+ _returnvalue_2 (`self.DropAvoidOffsetY`)))
                (`Pawn.AddControllerPitchInput` _maincharacter (* _returnvalue_2 -1.0))))))
        (:`Finished`
          ;;[1 0.5052 0.5052] 恢复默认
          (set `self.MaxRecoilY` 0.0)
          (set `self.DropAvoidOffsetY` 0.0)
          (set `self.MaxRecoilX` 0.0)
          (set `self.DropAvoidOffsetX` 0.0))))
    (:`then_2`
      (`self.StopUpBP`))))

(event `self.RecoilCameraShake`)

(event `self.RecoilHalfway`
  ;[1 1 1] 后坐力回落
  (goto _label_3 :!via `Stop`))

(event `self.ReceiveTick`
  (params (DeltaSeconds :type "Float (single-precision)"))
  ;[1 1 1] 后坐力枪身前后抖动
  (`|ExecutionSequence`
    (:`then_0`
      (bind _output_get (set `self.Anim_CurrentRecoilOffset` (`KismetMathLibrary.TInterpTo` (stale _output_get) (`KismetMathLibrary.MakeTransform` (0.0 0.0 0.0)) DeltaSeconds 10.0)))
      (bind _output_get_2 (set `self.Anim_RecoilOffset` (`KismetMathLibrary.TInterpTo` (stale _output_get_2) (`self.Anim_CurrentRecoilOffset`) DeltaSeconds 10.0))))
    (:`then_1`
      (`KismetSystemLibrary.PrintString` (`KismetStringLibrary.Conv_IntToString` (`self.CurrentBulletNum`))))))

(fn `RelordUpdate`
  (params (CurrentBulletNum :type Integer) (TotalBulletNum :type Integer)))

(fn `UserConstructionScript`
  (`parent.UserConstructionScript`))