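; AK47 weapon pickup that gives the main character the rifle when touched.
; Its sphere overlap casts to BP_MainCharacter, stores it and calls GiveItem, which adds the configured item type and count to the character's inventory component and destroys the pickup.
; The overlap handler then sets the character's weapon Blueprint to BP_WeaponAK47, after the destroy call.
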(event `self.Sphere.OnComponentBeginOverlap`
  (params (OverlappedComponent :type "PrimitiveComponent Object Reference") (OtherActor :type "Actor Object Reference") (OtherComp :type "PrimitiveComponent Object Reference") (OtherBodyIndex :type Integer) (bFromSweep :type Boolean) (SweepResult :type "HitResult Structure (by ref)"))
  (bind _asbp_main_character (cast `/Game/Game/Core/BP_MainCharacter` OtherActor))
  (set `self.PlayerCollection` _asbp_main_character)
  (`self.GiveItem`)
  (`MainCharacter.SetWeaponBP` (`self.PlayerCollection`) "/Game/Game/Weapon/WeaponChild/BP_WeaponAK47.BP_WeaponAK47_C"))

(event `GiveItem`
  (`InventoryComponent.AddInventoryItem` (`FPS_NetworkCharacter.InventoryComponent` (`self.PlayerCollection`)) (make `InventoryItem` (`self.ItemType`) (`self.Count`)))
  (`self.K2_DestroyActor`))

(fn `UserConstructionScript`)