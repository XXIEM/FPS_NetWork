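; Base weapon pickup actor that gives its weapon to the main character on sphere overlap.
; It maps the item's weapon type (main, secondary or knife) to a slot and sets it as the character's current inventory index.
; The character then initializes the weapon Blueprint at that index.
; Finally, the pickup adds the item and count to the inventory component at that index and destroys itself.
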(event `self.Sphere.OnComponentBeginOverlap`
  (params (OverlappedComponent :type "PrimitiveComponent Object Reference") (OtherActor :type "Actor Object Reference") (OtherComp :type "PrimitiveComponent Object Reference") (OtherBodyIndex :type Integer) (bFromSweep :type Boolean) (SweepResult :type "HitResult Structure (by ref)"))
  (bind _asbp_main_character (cast `/Game/Game/Core/BP_MainCharacter` OtherActor))
  (set `self.PlayerCollection` _asbp_main_character)
  (set `self.In Weapon` (`WeaponItem.WeaponBP` (`self.ItemType`)))
  (`self.InitWeaponBP`)
  (`self.GiveItemUI`))

(event `GiveItemUI`
  (bind _playercollection (`self.PlayerCollection`))
  (`InventoryComponent.AddInventoryItemByIndex` (`FPS_NetworkCharacter.InventoryComponent` _playercollection) (make `InventoryItem` (`self.ItemType`) (`self.Count`)) (`FPS_NetworkCharacter.CurrentInventoryIndex` _playercollection))
  (`self.K2_DestroyActor`))

(event `InitWeaponBP`
  (bind _playercollection (`self.PlayerCollection`))
  (bind _weapontype (`WeaponItem.WeaponType` (`self.ItemType`)))
  (if (`|EnumEquality` _weapontype "MainWeapon")
    (set `FPS_NetworkCharacter.CurrentInventoryIndex` 0 _playercollection)
    (`MainCharacter.InitWeaponBP` (`self.PlayerCollection`) (`self.In Weapon`) (`FPS_NetworkCharacter.CurrentInventoryIndex` _playercollection) :!label _label)
    (elif (`|EnumEquality` _weapontype "SecondaryWeapon")
      (set `FPS_NetworkCharacter.CurrentInventoryIndex` 1 _playercollection)
      (goto _label)
      (elif (`|EnumEquality` _weapontype "Knife")
        (set `FPS_NetworkCharacter.CurrentInventoryIndex` 2 _playercollection)
        (goto _label)))))

(fn `UserConstructionScript`)