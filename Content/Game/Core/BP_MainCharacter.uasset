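; Main player character Blueprint that supplies weapon motion curves, aim blending and the main HUD.
; WeaponMove starts walk and sprint timelines that write sway curve values, and hides the head bone for the locally controlled player.
; Start and end aim events both play one timeline from the start to drive AimMultiplier.
; AddMainUI creates the main widget and caches its reload sub-widget.
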(event `SprintWave`
  (bind (_direction _weaponmovecurve) (`Timeline|WeaponSprintWave`)
    (:`Update`
      (set `self.Weapon Sprint Curve` _weaponmovecurve))))

(event `WalkWave`
  (bind (_direction _weaponmovecurve) (`Timeline|WeaponWalkWave`)
    (:`Update`
      (set `self.Weapon Walk Curve` _weaponmovecurve))))

(event `self.WeaponMove`
  (`|ExecutionSequence`
    (:`then_0`
      (`TimelineComponent.SetTimelineLengthMode` (`self.WeaponWalkWave`) "TL_LastKeyFrame")
      (`TimelineComponent.SetTimelineLengthMode` (`self.WeaponSprintWave`) "TL_LastKeyFrame")
      (`self.WalkWave`)
      (`self.SprintWave`))
    (:`then_1`
      (if (`self.IsLocallyControlled`)
        (`SkinnedMeshComponent.HideBoneByName` (`self.Mesh`) "head" "PBO_None")))))

(event `self.AddMainUI`
  (bind _returnvalue (`|CreateWidget` "/Game/Game/UI/UW_MainUI.UW_MainUI_C" (`GameplayStatics.GetPlayerController` 0)))
  (`UserWidget.AddToViewport` _returnvalue 0)
  (set `self.UI_Relord` (`/Game/Game/UI/UW_MainUI.UW_Relord` _returnvalue)))

(event `self.StartAimSwitchCurve`
  (bind (_direction _aimmultiplier) (`Timeline|Timeline` :!via `PlayFromStart` :!label _label)
    (:`Update`
      (set `self.Aim Multiplier` _aimmultiplier))))

(event `self.EndAimSwitchCurve`
  (goto _label :!via `PlayFromStart`))

(fn `UserConstructionScript`
  (`parent.UserConstructionScript`))