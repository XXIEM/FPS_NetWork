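; BP_AddBullet is an ammo pickup that refills the main character's current weapon on touch.
; A sphere overlap finds the gun in the character's current inventory slot and adds one magazine's worth (MaxCurrentBulletNum) to its total reserve.
; It then updates the reload UI on the first player's HUD and destroys itself.
; Any failed character, weapon or HUD cast leaves the pickup untouched.
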(event `self.Sphere.OnComponentBeginOverlap`
  (params (OverlappedComponent :type "PrimitiveComponent Object Reference") (OtherActor :type "Actor Object Reference") (OtherComp :type "PrimitiveComponent Object Reference") (OtherBodyIndex :type Integer) (bFromSweep :type Boolean) (SweepResult :type "HitResult Structure (by ref)"))
  (bind _asbp_main_character (cast `/Game/Game/Core/BP_MainCharacter` OtherActor))
  (bind _asbp_weapon_base (cast `/Game/Game/Weapon/BP_WeaponBase` (`|GetArrayItem` (`MainCharacter.ExistGun` _asbp_main_character) (`FPS_NetworkCharacter.CurrentInventoryIndex` _asbp_main_character))))
  (bind _asbp_main_hud (cast `/StickyNotesSystem/BP_MainHUD` (`PlayerController.GetHUD` (`GameplayStatics.GetPlayerController` 0))))
  (bind _output_get (set `WeaponBase.TotalBulletNum` (+ (`WeaponBase.TotalBulletNum` _asbp_weapon_base) (`WeaponBase.MaxCurrentBulletNum` _asbp_weapon_base)) _asbp_weapon_base))
  (message `/Game/Game/Weapon/BPI_BulletRelord.RelordUpdate` (`MainHUD.RelordUI` _asbp_main_hud) (`WeaponBase.CurrentBulletNum` _asbp_weapon_base) _output_get)
  (`self.K2_DestroyActor`))

(fn `UserConstructionScript`)